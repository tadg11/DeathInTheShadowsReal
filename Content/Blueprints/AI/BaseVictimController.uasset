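; BaseVictimController is an AI controller for victim characters that runs the BT_Victim behavior tree.
; On BeginPlay it starts the tree, waits briefly, then stores the controlled pawn's location in the Home blackboard key.
; Its PawnSensing component sets the Alert key to true when it sees the player character; nothing here clears it.
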(event OnSeePawn(PawnSensing)
  (params (Pawn :type Pawn%20Object%20Reference))
  (bind _blackboard (Variables|Default|GetBlackboard))
  (if (== Pawn (Game|GetPlayerCharacter 0))
    (Utilities|IsValid _blackboard
      (:Is%20Valid
        (AI|Components|Blackboard|SetValueasBool _blackboard (Utilities|Name|MakeLiteralName "Alert") true)))))

(event EventBeginPlay
  (AI|RunBehaviorTree "/Game/Blueprints/AI/BT_Victim.BT_Victim")
  (Utilities|FlowControl|Delay 0.2)
  (AI|Components|Blackboard|SetValueasVector (Variables|Default|GetBlackboard) (Utilities|Name|MakeLiteralName "Home") (Transformation|GetActorLocation (Pawn|GetControlledPawn))))

(event EventTick
  (params (DeltaSeconds :type Float%20%28single-precision%29)))

(fn ConstructionScript)