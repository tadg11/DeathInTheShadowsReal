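; Base victim character that the game counts as a kill when it takes damage.
; On BeginPlay it randomly picks a formal or casual skeletal mesh.
; The first damage of any amount marks it dead, notifies the game mode's kill counter, and turns on mesh physics with an impulse away from the player.
; Death also disables movement, gravity on the movement component and capsule collision.
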(event EventBeginPlay
  (Components|SkeletalMesh|SetSkeletalMeshAsset (Variables|Character|GetMesh) (select (Math|Random|RandomBool) "/Game/Artwork/SkeletalMeshes/Women/Formal/Formal.Formal" "/Game/Artwork/SkeletalMeshes/Women/Casual/Casual.Casual")))

(event Collision|EventActorBeginOverlap
  (params (OtherActor :type Actor%20Object%20Reference)))

(event EventTick
  (params (DeltaSeconds :type Float%20%28single-precision%29)))

(event Game|Damage|EventAnyDamage
  (params (Damage :type Float%20%28single-precision%29) (DamageType :type Damage%20Type%20Object%20Reference) (InstigatedBy :type Controller%20Object%20Reference) (DamageCauser :type Actor%20Object%20Reference))
  (bind _mesh (Variables|Character|GetMesh))
  (bind _charactermovement (Variables|Character|GetCharacterMovement))
  (if (not (Variables|Default|GetDead))
    (Variables|Default|SetDead true)
    (Class|GMInterface|CountKills(Message) (Game|GetGameMode))
    (Physics|SetSimulatePhysics _mesh true)
    (Physics|AddImpulse _mesh (* (- (Transformation|GetActorLocation) (Transformation|GetActorLocation (Game|GetPlayerCharacter 0))) 1e+01) "None" true)
    (Pawn|Components|CharacterMovement|DisableMovement _charactermovement)
    (Variables|/Script/Engine.CharacterMovementComponent|SetGravityScale _charactermovement 0.0)
    (Collision|SetCollisionEnabled (Variables|Collision|GetCapsuleComponent) "NoCollision")))

(fn ConstructionScript)