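; BP_BaseCop is a cop AI character that picks one of two meshes at random and watches for the player with a vision cone.
; Player overlap notifies the controller and plays a timeline that shifts the cone's dynamic material from orange toward red.
; Completing the timeline forward tells the game mode to kill the player, while leaving the cone reverses it.
; Patrol assignments are forwarded to the controller.
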(event OnComponentBeginOverlap(Vision)
  (params (OverlappedComponent :type Primitive%20Component%20Object%20Reference) (OtherActor :type Actor%20Object%20Reference) (OtherComp :type Primitive%20Component%20Object%20Reference) (OtherBodyIndex :type Integer) (bFromSweep :type Boolean) (SweepResult :type Hit%20Result%20Structure%20%28by%20ref%29))
  (if (== OtherActor (Game|GetPlayerCharacter 0))
    (Class|AiInterface|EnemySpotted(Message) (Pawn|GetController))
    (bind (_direction _newtrack_0) (Timeline|AlertLine Play)
      (:Update
        (Rendering|Material|SetVectorParameterValue (Variables|Default|GetVisionmatt) "Alertness" (Math|Color|Lerp(LinearColor) "(R=1.000000,G=0.430350,B=0.000000,A=1.000000)" "(R=1.000000,G=0.048789,B=0.000000,A=1.000000)" _newtrack_0) :!class /Script/Engine.MaterialInstanceDynamic))
      (:Finished
        (switch Utilities|FlowControl|Switch|SwitchonETimelineDirection _direction
          (:Forward
            (Class|GMInterface|KillPlayer(Message) (Game|GetGameMode))))))))

(event OnComponentEndOverlap(Vision)
  (params (OverlappedComponent :type Primitive%20Component%20Object%20Reference) (OtherActor :type Actor%20Object%20Reference) (OtherComp :type Primitive%20Component%20Object%20Reference) (OtherBodyIndex :type Integer))
  (if (== OtherActor (Game|GetPlayerCharacter 0))
    (bind (_direction _newtrack_0) (Timeline|AlertLine Reverse)
      (:Update
        (Rendering|Material|SetVectorParameterValue (Variables|Default|GetVisionmatt) "Alertness" (Math|Color|Lerp(LinearColor) "(R=1.000000,G=0.430350,B=0.000000,A=1.000000)" "(R=1.000000,G=0.048789,B=0.000000,A=1.000000)" _newtrack_0) :!class /Script/Engine.MaterialInstanceDynamic))
      (:Finished
        (switch Utilities|FlowControl|Switch|SwitchonETimelineDirection _direction
          (:Forward
            (Class|GMInterface|KillPlayer(Message) (Game|GetGameMode))))))))

(event EventBeginPlay
  (Components|SkeletalMesh|SetSkeletalMeshAsset (Variables|Character|GetMesh) (select (Math|Random|RandomBool) "/Game/Artwork/SkeletalMeshes/Women/Soldier/Soldier.Soldier" "/Game/Artwork/SkeletalMeshes/Women/Sci-Fi/SciFi.SciFi"))
  (bind _returnvalue (Rendering|Material|CreateDynamicMaterialInstance (Variables|Default|GetVision) 0 "/Game/Artwork/Materials/VisionCone.VisionCone" "None" :!class /Script/Engine.PrimitiveComponent))
  (Variables|Default|SetVisionmatt _returnvalue))

(event Collision|EventActorBeginOverlap
  (params (OtherActor :type Actor%20Object%20Reference)))

(event EventTick
  (params (DeltaSeconds :type Float%20%28single-precision%29)))

(event EventAssignPatrol
  (params (Patrol :type Array%20of%20Vectors))
  (Class|AiInterface|AssignPatrol(Message) (Pawn|GetController) Patrol))

(fn ConstructionScript)

(fn NewPatrolPoint
  (return "0, 0, 0"))