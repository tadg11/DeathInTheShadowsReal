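; A collectible pickup actor that the player gathers by overlapping it.
; On first overlap with the player character it sets IsPickedUp, hides its Cube and calls CountPickupsMessage on the game mode.
; A ResetLevel event respawns it by clearing the flag and showing the Cube again, so the actor is reused rather than destroyed.
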(event EventBeginPlay)

(event Collision|EventActorBeginOverlap
  (params (OtherActor :type Actor%20Object%20Reference))
  (if (== OtherActor (Game|GetPlayerCharacter 0))
    (if (not (Variables|Default|GetIsPickedUp))
      (CallFunction|Collect))))

(event EventTick
  (params (DeltaSeconds :type Float%20%28single-precision%29)))

(event EventResetLevel
  (CallFunction|Respawn))

(fn ConstructionScript)

(fn Collect
  (bind _output_get (Variables|Default|SetIsPickedUp true))
  (if _output_get
    (Development|SetHiddeninGame (Variables|Default|GetCube) _output_get false)
    (Class|GMInterface|CountPickups(Message) (Game|GetGameMode))))

(fn Respawn
  (Variables|Default|SetIsPickedUp false)
  (Development|SetHiddeninGame (Variables|Default|GetCube) false false))