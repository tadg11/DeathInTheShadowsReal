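; In-level game rules that run a timed, graded level attempt from start through player death to end screen.
; Init tallies possible kills and points from spawners and collectibles, then a looping millisecond timer event drives the clock.
; KillPlayer resets level actors, counters and timer for a retry.
; EndLevel passes a DoOnce to grade time, kills and score, asynchronously merge personal bests into the save slot, and show HUD results.
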(event Custom|Init
  (bind _asbase_game_instance (Utilities|Casting|CastToBaseGameInstance (Game|GetGameInstance)))
  (Variables|Default|SetCurrent%20Level (Variables|/Game/Blueprints/GameRules/BaseGameInstance.BaseGameInstance_C|GetCurrentLevel _asbase_game_instance))
  (CallFunction|PreGame))

(event Custom|PreGame
  (CallFunction|CountPotentialKills)
  (CallFunction|CountPotentialScore)
  (CallFunction|InGame))

(event Custom|In%20Game
  (CallFunction|StartTimer))

(event Custom|End%20Game
  (bind _returnvalue (Game|GetPlayerController 0))
  (bind _miliseconds (Variables|Default|GetMiliseconds))
  (bind _seconds (Variables|Default|GetSeconds))
  (bind _minutes (Variables|Default|GetMinutes))
  (Utilities|FlowControl|DoOnce false
    (:Completed
      (Input|SetIgnoreLookInput _returnvalue true)
      (Input|SetIgnoreMoveInput _returnvalue true)
      (Variables|/Script/Engine.PlayerController|SetbShowMouseCursor _returnvalue true)
      (Variables|Default|SetTimeInSeconds (+ (* (Math|Conversions|ToFloat(Integer) (Variables|Default|GetMinutes)) 6e+01) (Math|Conversions|ToFloat(Integer) (Variables|Default|GetSeconds)) (/ (Math|Conversions|ToFloat(Integer) (Variables|Default|GetMiliseconds)) 1e+03)))
      (CallFunction|CalcScore)
      (Variables|Default|SetLevelData (Utilities|Struct|MakeLevelData _miliseconds _seconds _minutes (Utilities|String|Append (Utilities|String|ToString(Integer) _minutes) ":" (Utilities|String|ToString(Integer) _seconds) ":" (Utilities|String|ToString(Integer) _miliseconds)) (Variables|Default|GetKills) (Variables|Default|GetPoints) (Variables|Default|GetSecrets) (Variables|Default|GetGrade)))
      (CallFunction|Compare&Save)
      (CallFunction|PostGame))))

(event Custom|PostGame
  (Class|UIInterface|ShowEndScreen(Message) (HUD|GetHUD (Game|GetPlayerController 0)) (Variables|Default|GetLevelData) (Variables|Default|GetNewPB) (Variables|Default|GetTime) (Variables|Default|GetKillGrade) (Variables|Default|GetScore)))

(event Custom|StartTimer
  ;[1 1 1] tIMER
  (bind _returnvalue (Utilities|Time|SetTimerbyEvent (delegate Custom|GameClock) 0.001 true)))

(event Custom|ResetTimer
  ;[1 1 1] tIMER
  (Utilities|Time|ClearandInvalidateTimerbyHandle (stale Custom|StartTimer _returnvalue))
  (Variables|Default|SetSeconds 0)
  (Variables|Default|SetMinutes 0)
  (Variables|Default|SetMiliseconds 0))

(event Custom|GameClock
  ;[1 1 1] tIMER
  (if (>= (+ (Variables|Default|GetMiliseconds) 1) 1000)
    (Variables|Default|SetMiliseconds 0)
    (if (>= (+ (Variables|Default|GetSeconds) 1) 60)
      (Variables|Default|SetSeconds 0)
      (Variables|Default|SetMinutes (+ (Variables|Default|GetMinutes) 1))
      (else
        (Variables|Default|SetSeconds (+ (Variables|Default|GetSeconds) 1))))
    (else
      (Variables|Default|SetMiliseconds (+ (Variables|Default|GetMiliseconds) 1)))))

(event Custom|CalcScore
  (Variables|Default|SetPoints (+ (* (Variables|Default|GetKills) 100) (* (Variables|Default|GetPickups) 50)))
  (Variables|Default|SetTime (Utilities|CompareTimes))
  (Variables|Default|SetKillGrade (Utilities|CompareKills))
  (Variables|Default|SetScore (Utilities|ComparePoints))
  (Variables|Default|SetGrade (Utilities|AverageGrades))
  (Development|PrintString (Utilities|String|ToString(Float) (/ (+ (Math|Conversions|ToFloat(Byte) (Variables|Default|GetTime)) (Math|Conversions|ToFloat(Byte) (Variables|Default|GetKillGrade)) (Math|Conversions|ToFloat(Byte) (Variables|Default|GetScore))) 3.0))))

(event Custom|Compare%20&%20Save
  (bind _current_level (Variables|Default|GetCurrent%20Level))
  (bind _grade (Variables|Default|GetGrade))
  (bind _leveldata (Variables|Default|GetLevelData))
  (bind _grade_2 (Variables|Default|GetGrade))
  (bind _secrets (Variables|Default|GetSecrets))
  (bind _kills (Variables|Default|GetKills))
  (bind _points (Variables|Default|GetPoints))
  (bind _current_level_2 (Variables|Default|GetCurrent%20Level))
  (bind (_savegame _bsuccess) (|AsyncLoadGamefromSlot "Test" 2)
    (:Completed
      (if _bsuccess
        (bind _assave_file (Utilities|Casting|CastToSaveFile _savegame))
        (bind _output_get (Variables|Default|SetNewPB (Utilities|CheckPersonalBest (Utilities|Array|Get(acopy) (Variables|/Game/Blueprints/GameRules/SaveFile.SaveFile_C|GetLevelBests _assave_file) (Variables|Default|GetCurrent%20Level)))))
        (if _output_get
          (Utilities|Array|SetArrayElem (Variables|/Game/Blueprints/GameRules/SaveFile.SaveFile_C|GetLevelBests _assave_file) _current_level (Utilities|Struct|MakeLevelData (.miliseconds _leveldata) (.seconds _leveldata) (.minutes _leveldata) (.time _leveldata) (.kills _leveldata) (.score _leveldata) (.secrets _leveldata) (select (> (Math|Conversions|ToFloat(Byte) _grade) (Math|Conversions|ToFloat(Byte) (.Grade (Utilities|Struct|BreakLevelData (Utilities|Array|Get(acopy) (Variables|/Game/Blueprints/GameRules/SaveFile.SaveFile_C|GetLevelBests _assave_file) (Variables|Default|GetCurrent%20Level)))))) _grade (.Grade (Utilities|Struct|BreakLevelData (Utilities|Array|Get(acopy) (Variables|/Game/Blueprints/GameRules/SaveFile.SaveFile_C|GetLevelBests _assave_file) (Variables|Default|GetCurrent%20Level)))))))
          (else
            (Utilities|Array|SetArrayElem (Variables|/Game/Blueprints/GameRules/SaveFile.SaveFile_C|GetLevelBests _assave_file) _current_level (Utilities|Struct|MakeLevelData (.Miliseconds (Utilities|Struct|BreakLevelData (Utilities|Array|Get(acopy) (Variables|/Game/Blueprints/GameRules/SaveFile.SaveFile_C|GetLevelBests _assave_file) (Variables|Default|GetCurrent%20Level)))) (.Seconds (Utilities|Struct|BreakLevelData (Utilities|Array|Get(acopy) (Variables|/Game/Blueprints/GameRules/SaveFile.SaveFile_C|GetLevelBests _assave_file) (Variables|Default|GetCurrent%20Level)))) (.Minutes (Utilities|Struct|BreakLevelData (Utilities|Array|Get(acopy) (Variables|/Game/Blueprints/GameRules/SaveFile.SaveFile_C|GetLevelBests _assave_file) (Variables|Default|GetCurrent%20Level)))) (.Time (Utilities|Struct|BreakLevelData (Utilities|Array|Get(acopy) (Variables|/Game/Blueprints/GameRules/SaveFile.SaveFile_C|GetLevelBests _assave_file) (Variables|Default|GetCurrent%20Level)))) (Math|Integer|SelectInt _kills (.Kills (Utilities|Struct|BreakLevelData (Utilities|Array|Get(acopy) (Variables|/Game/Blueprints/GameRules/SaveFile.SaveFile_C|GetLevelBests _assave_file) (Variables|Default|GetCurrent%20Level)))) (> _kills (.Kills (Utilities|Struct|BreakLevelData (Utilities|Array|Get(acopy) (Variables|/Game/Blueprints/GameRules/SaveFile.SaveFile_C|GetLevelBests _assave_file) (Variables|Default|GetCurrent%20Level)))))) (Math|Integer|SelectInt _points (.Score (Utilities|Struct|BreakLevelData (Utilities|Array|Get(acopy) (Variables|/Game/Blueprints/GameRules/SaveFile.SaveFile_C|GetLevelBests _assave_file) (Variables|Default|GetCurrent%20Level)))) (> _points (.Score (Utilities|Struct|BreakLevelData (Utilities|Array|Get(acopy) (Variables|/Game/Blueprints/GameRules/SaveFile.SaveFile_C|GetLevelBests _assave_file) (Variables|Default|GetCurrent%20Level)))))) (Math|Integer|SelectInt _secrets (.Secrets (Utilities|Struct|BreakLevelData (Utilities|Array|Get(acopy) (Variables|/Game/Blueprints/GameRules/SaveFile.SaveFile_C|GetLevelBests _assave_file) (Variables|Default|GetCurrent%20Level)))) (> _secrets (.Secrets (Utilities|Struct|BreakLevelData (Utilities|Array|Get(acopy) (Variables|/Game/Blueprints/GameRules/SaveFile.SaveFile_C|GetLevelBests _assave_file) (Variables|Default|GetCurrent%20Level)))))) (select (> (Math|Conversions|ToFloat(Byte) _grade_2) (Math|Conversions|ToFloat(Byte) (.Grade (Utilities|Struct|BreakLevelData (Utilities|Array|Get(acopy) (Variables|/Game/Blueprints/GameRules/SaveFile.SaveFile_C|GetLevelBests _assave_file) (Variables|Default|GetCurrent%20Level)))))) _grade_2 (.Grade (Utilities|Struct|BreakLevelData (Utilities|Array|Get(acopy) (Variables|/Game/Blueprints/GameRules/SaveFile.SaveFile_C|GetLevelBests _assave_file) (Variables|Default|GetCurrent%20Level)))))))))
        (if (>= _current_level_2 (Variables|/Game/Blueprints/GameRules/SaveFile.SaveFile_C|GetCurrentLevel _assave_file))
          (Variables|/Game/Blueprints/GameRules/SaveFile.SaveFile_C|SetCurrentLevel _assave_file _current_level_2))
        (|AsyncSaveGametoSlot _savegame "Test" 2)
        (else
          (bind _returnvalue (SaveGame|CreateSaveGameObject "/Game/Blueprints/GameRules/SaveFile.SaveFile_C"))
          (bind _savegame_2 (|AsyncSaveGametoSlot _returnvalue "Test" 2)
            (:then
              (bind _assave_file_2 (Utilities|Casting|CastToSaveFile _savegame_2))
              (Variables|Default|SetNewPB true)
              (Utilities|Array|SetArrayElem (Variables|/Game/Blueprints/GameRules/SaveFile.SaveFile_C|GetLevelBests _assave_file_2) (Variables|Default|GetCurrent%20Level) (Variables|Default|GetLevelData))
              (if (>= _current_level_2 (Variables|/Game/Blueprints/GameRules/SaveFile.SaveFile_C|GetCurrentLevel _assave_file_2))
                (Variables|/Game/Blueprints/GameRules/SaveFile.SaveFile_C|SetCurrentLevel _assave_file_2 _current_level_2))
              (|AsyncSaveGametoSlot _savegame_2 "Test" 2))))))))

(event EventBeginPlay
  (CallFunction|Init))

(event EventTick
  (params (DeltaSeconds :type Float%20%28single-precision%29)))

(event EventCountSecrets
  ;[1 1 1] Count Items
  (Variables|Default|SetSecrets (+ (Variables|Default|GetSecrets) 1)))

(event EventCountPickups
  ;[1 1 1] Count Items
  (Variables|Default|SetPickups (+ (Variables|Default|GetPickups) 1)))

(event EventCountKills
  ;[1 1 1] Count Items
  (Variables|Default|SetKills (+ (Variables|Default|GetKills) 1)))

(event EventKillPlayer
  (bind _returnvalue (Game|GetPlayerController 0))
  (bind _miliseconds (Variables|Default|GetMiliseconds))
  (bind _seconds (Variables|Default|GetSeconds))
  (bind _minutes (Variables|Default|GetMinutes))
  ;[1 1 1] Reset levels
  (Class|GMInterface|KillPlayer(Message) (Game|GetPlayerCharacter 0))
  (Utilities|FlowControl|Sequence
    (:then_0
      (bind _outactors (Actor|GetAllActorsOfClass "/Game/Blueprints/LevelObjets/Collectible.Collectible_C"))
      (for _array_element _outactors
        (Class|GMInterface|ResetLevel(Message) _array_element))
      (bind _outactors_2 (Actor|GetAllActorsOfClass "/Game/Artwork/Decals/DeathSplat.DeathSplat_C"))
      (for _array_element_2 _outactors_2
        (Actor|DestroyActor _array_element_2)))
    (:then_1
      (bind _outactors_3 (Actor|GetAllActorsOfClass "/Game/Blueprints/LevelObjets/Spawners/VictimSpawner.VictimSpawner_C"))
      (for _array_element_3 _outactors_3
        (Class|GMInterface|ResetLevel(Message) _array_element_3))
      (bind _outactors_4 (Actor|GetAllActorsOfClass "/Game/Blueprints/LevelObjets/Spawners/CopSpawner.CopSpawner_C"))
      (for _array_element_4 _outactors_4
        (Class|GMInterface|ResetLevel(Message) _array_element_4)))
    (:then_2
      (Variables|Default|SetTimeInSeconds 0.0)
      (Variables|Default|SetPickups 0)
      (Variables|Default|SetKills 0)
      (Variables|Default|SetPoints 0)
      (CallFunction|ResetTimer))
    (:then_3
      (CallFunction|InGame))
    (:then_4
      (Utilities|FlowControl|DoOnce false) ; enters at Reset
    )))

(event EventEndLevel
  (CallFunction|EndGame))

(fn ConstructionScript)

(fn CountPotentialKills
  (bind _outactors (Actor|GetAllActorsOfClass "/Game/Blueprints/LevelObjets/Spawners/VictimSpawner.VictimSpawner_C"))
  (for _array_element _outactors
    (Variables|Default|SetTotalNPCS (+ (Variables|Default|GetTotalNPCS) 1)))
  (bind _outactors_2 (Actor|GetAllActorsOfClass "/Game/Blueprints/LevelObjets/Spawners/CopSpawner.CopSpawner_C"))
  (for _array_element_2 _outactors_2
    (Variables|Default|SetTotalNPCS (+ (Variables|Default|GetTotalNPCS) 1))))

(fn CountPotentialScore
  (bind _outactors (Actor|GetAllActorsOfClass "/Game/Blueprints/LevelObjets/Collectible.Collectible_C"))
  (for (_ _array_index) _outactors
    (Variables|Default|SetPotentialPoints (+ (Variables|Default|GetPotentialPoints) (* _array_index 50))))
  (Variables|Default|SetPotentialPoints (+ (Variables|Default|GetPotentialPoints) (* (Variables|Default|GetTotalNPCS) 100))))